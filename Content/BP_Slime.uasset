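; BP_Slime is a patrolling enemy that kills BP_Player on overlap by calling its Die function.
; From BeginPlay, a timeline ping-pongs between play and reverse, its alpha scaled by SlimeSpeed driving a swept offset along local Y each update.
; At each end it flips 180 degrees, so the same local offset carries it back the other way.
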(event `self.ReceiveActorBeginOverlap`
  (params (OtherActor :type "Actor Object Reference"))
  (bind _asbp_player (cast `/Game/Blueprints/Player/BP_Player` OtherActor))
  (`/Game/Blueprints/Player/BP_Player.Die` _asbp_player))

(event `MoveSlimeForward`
  (bind (_direction _offsetalpha) (`Timeline|SlimeTimeline` :!label _label)
    (:`Update`
      (`self.K2_AddActorLocalOffset` (`KismetMathLibrary.MakeVector` 0.0 (* _offsetalpha (`self.SlimeSpeed`))) true))
    (:`Finished`
      (switch `ETimelineDirection` _direction
        (:`Forward`
          (`self.MoveSlimeBack`))
        (:`Backward`
          (`self.MoveSlimeForward`)))
      (`self.K2_AddActorLocalRotation` (struct :`Yaw` 180.0)))))

(event `self.ReceiveBeginPlay`
  (`self.MoveSlimeForward`))

(event `MoveSlimeBack`
  (goto _label :!via `Reverse`))

(fn `UserConstructionScript`)