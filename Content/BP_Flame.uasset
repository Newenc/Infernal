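; BP_Flame is a hazard that switches a flame on and off and kills the player on contact.
; A looping timer started on BeginPlay flips IsFlameOn every two seconds, toggling the Niagara effect's visibility together with the Capsule's query collision.
; Any BP_Player that begins overlapping the Capsule has Die called on it.
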(event `self.Capsule.OnComponentBeginOverlap`
  (params (OverlappedComponent :type "PrimitiveComponent Object Reference") (OtherActor :type "Actor Object Reference") (OtherComp :type "PrimitiveComponent Object Reference") (OtherBodyIndex :type Integer) (bFromSweep :type Boolean) (SweepResult :type "HitResult Structure (by ref)"))
  (bind _asbp_player (cast `/Game/Blueprints/Player/BP_Player` OtherActor))
  (`/Game/Blueprints/Player/BP_Player.Die` _asbp_player))

(event `self.ReceiveBeginPlay`
  ; Enable/disable flame
  (`KismetSystemLibrary.K2_SetTimerDelegate` (delegate `ToggleFlameEvent`) 2.0 true))

(event `ToggleFlameEvent`
  ; Enable/disable flame
  (set `self.isFlameOn` (not (`self.isFlameOn`)))
  (if (`self.isFlameOn`)
    (`SceneComponent.SetVisibility` (`self.Niagara flame`) true false)
    (`PrimitiveComponent.SetCollisionEnabled` (`self.Capsule`) "QueryOnly")
    (else
      (`SceneComponent.SetVisibility` (`self.Niagara flame`) false false)
      (`PrimitiveComponent.SetCollisionEnabled` (`self.Capsule`) "NoCollision"))))

(fn `UserConstructionScript`)