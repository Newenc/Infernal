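; Game manager Blueprint that picks the background music to match the player's room progress.
; On BeginPlay, UpdateMusic reads the current room index from BP_GameInstance and maps every three rooms to a music index, clamped to four tracks.
; When that index differs from the current one, it swaps the sound on the first AmbientSound actor found in the level and fades it in.
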(event `self.ReceiveBeginPlay`
  (`self.UpdateMusic`))

(fn `UpdateMusic`
  (bind _asbp_game_instance (cast `/Game/BP_GameInstance` (`GameplayStatics.GetGameInstance`)))
  (set `self.LevelIndex` (`KismetMathLibrary.Clamp` (`KismetMathLibrary.FFloor` (`KismetMathLibrary.Conv_IntToDouble` (/ (`/Game/BP_GameInstance.CurrentRoomIndex` _asbp_game_instance) 3))) 0 3))
  (if (!= (`self.CurrentMusicIndex`) (`self.LevelIndex`))
    (bind _outactors (`GameplayStatics.GetAllActorsOfClass` "/Script/Engine.AmbientSound"))
    (bind _audiocomponent (`AmbientSound.AudioComponent` (`|GetArrayItem` _outactors)))
    (`AudioComponent.SetSound` _audiocomponent (`|GetArrayItem` (`self.MusicArray`) (`self.LevelIndex`)))
    (`AudioComponent.FadeIn` _audiocomponent 1.5 1.0 0.0 "Linear")
    (set `self.CurrentMusicIndex` (`self.LevelIndex`))))

(fn `UserConstructionScript`)