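; BP_Level_Portal is a portal that moves the player to a target point when they overlap its box collision.
; It also blends the first player controller's view to a target camera, then increments the current room index in BP_GameInstance.
; A HasTeleported flag, cleared after a one-second delay, blocks repeat increments but does not gate the teleport or camera switch.
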(event `self.BoxCollision1.OnComponentBeginOverlap`
  (params (OverlappedComponent :type "PrimitiveComponent Object Reference") (OtherActor :type "Actor Object Reference") (OtherComp :type "PrimitiveComponent Object Reference") (OtherBodyIndex :type Integer) (bFromSweep :type Boolean) (SweepResult :type "HitResult Structure (by ref)"))
  (bind _asbp_player (cast `/Game/Blueprints/Player/BP_Player` OtherActor))
  (`self.K2_SetActorLocation` _asbp_player (`self.TargetPoint`) false false)
  (`PlayerController.SetViewTargetWithBlend` (`GameplayStatics.GetPlayerController` 0) (`self.TargetCamera`) 0.2 "VTBlend_Linear" 0.0 false)
  ; Update CurrentLevelIndex
  (bind _asbp_game_instance (cast `/Game/BP_GameInstance` (`GameplayStatics.GetGameInstance`)))
  (if (not (`self.HasTeleported`))
    (bind _output_get (set `/Game/BP_GameInstance.CurrentRoomIndex` (+ (`/Game/BP_GameInstance.CurrentRoomIndex` _asbp_game_instance) 1) _asbp_game_instance))
    (set `self.HasTeleported` true)
    (`KismetSystemLibrary.PrintString` (`KismetStringLibrary.Conv_IntToString` _output_get) false false)
    (`KismetSystemLibrary.Delay` 1.0)
    (set `self.HasTeleported` false)))

(fn `UserConstructionScript`)